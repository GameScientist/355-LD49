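; Moving platform actor that slides back and forth along the world Y axis, with a randomized width per instance.
; PlayTimeline uses a FlipFlop to play or reverse the MoveToTheRight timeline, whose Position track sets absolute Y; it re-triggers itself on Finished and once on Update.
; The construction script randomizes cube width and a StartTimeline value; BeginPlay only calls SetNewTime, without starting PlayTimeline.
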(event `PlayTimeline`
  (bind (_returnvalue_x _returnvalue_y _returnvalue_z) (`KismetMathLibrary.BreakVector` (`self.K2_GetActorLocation`)))
  ;[1 1 1] The timeline updates the location of the platform by making it repeatedly move left and right.
  (`/Engine/EditorBlueprintResources/StandardMacros.FlipFlop`
    (:`A`
      (bind (_direction _position) (`Timeline|MoveToTheRight` :`NewTime` (`self.startTimeline`) :!label _label)
        (:`Update`
          (`self.K2_SetActorLocation` (`KismetMathLibrary.MakeVector` _returnvalue_x _position _returnvalue_z))
          (`/Engine/EditorBlueprintResources/StandardMacros.DoOnce` false
            (:`Completed`
              _)))
        (:`Finished`
          _))
      (`self.PlayTimeline`))
    (:`B`
      (goto _label :!via `Reverse`))))

(event `self.ReceiveBeginPlay`
  ;[1 1 1] The timeline updates the location of the platform by making it repeatedly move left and right.
  (goto _label :!via `SetNewTime`))

(fn `UserConstructionScript`
  ;[1 1 1] A random width is set for each instance of this platform.
  (`SceneComponent.SetWorldScale3D` (`self.Cube`) (`KismetMathLibrary.MakeVector` 3.0 (`KismetMathLibrary.RandomFloatInRange` 2.0 3.0) 1.0))
  (set `self.startTimeline` (`KismetMathLibrary.RandomFloat`)))