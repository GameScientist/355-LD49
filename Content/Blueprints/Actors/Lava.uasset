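; Lava actor that rises beneath the player as a kill hazard, pushing them to keep climbing.
; Each tick it snaps to a fixed gap below the player and resets its speed if it falls too far behind; otherwise it accelerates upward.
; One overlap box destroys falling, moving and rotating platforms, while a separate kill box triggers the player's game over.
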(event `self.BlockDestroyBox.OnComponentBeginOverlap`
  (params (OverlappedComponent :type "PrimitiveComponent Object Reference") (OtherActor :type "Actor Object Reference") (OtherComp :type "PrimitiveComponent Object Reference") (OtherBodyIndex :type Integer) (bFromSweep :type Boolean) (SweepResult :type "HitResult Structure (by ref)"))
  ;[1 1 1 1 21] Blocks are destroyed on overlap with this component.
  (bind _asfalling_block (cast `/Game/Blueprints/Actors/FallingBlock` OtherActor)
    (:`then`
      (`self.K2_DestroyActor` _asfalling_block))
    (:`CastFailed`
      (bind _asmoving_platform (cast `/Game/Blueprints/Actors/MovingPlatform` OtherActor)
        (:`then`
          (`self.K2_DestroyActor` _asmoving_platform))
        (:`CastFailed`
          (bind _asrotating_platform (cast `/Game/Blueprints/Actors/RotatingPlatform` OtherActor))
          (`self.K2_DestroyActor` _asrotating_platform))))))

(event `self.PlayerKillBox.OnComponentBeginOverlap`
  (params (OverlappedComponent :type "PrimitiveComponent Object Reference") (OtherActor :type "Actor Object Reference") (OtherComp :type "PrimitiveComponent Object Reference") (OtherBodyIndex :type Integer) (bFromSweep :type Boolean) (SweepResult :type "HitResult Structure (by ref)"))
  ;[1 1 1 1 22] The player kill box kills the player on overlap.
  (bind _asplayer_pawn (cast `/Game/Blueprints/Actors/PlayerPawn` OtherActor))
  (`/Game/Blueprints/Actors/PlayerPawn.Game Over` _asplayer_pawn))

(event `self.ReceiveTick`
  (params (DeltaSeconds :type "Float (single-precision)"))
  (bind (_returnvalue_x _returnvalue_y _returnvalue_z) (`KismetMathLibrary.BreakVector` (`self.K2_GetActorLocation`)))
  ;[1 1 1 1 21] Updates the position of the lava.
  ;;[1 1 1] Every tick, the distance between the player and the lava is compared.
  (bind _asplayer_pawn (cast `/Game/Blueprints/Actors/PlayerPawn` (`GameplayStatics.GetPlayerCharacter` 0)))
  (bind (_returnvalue_x_2 _returnvalue_y_2 _returnvalue_z_2) (`KismetMathLibrary.BreakVector` (`self.K2_GetActorLocation` _asplayer_pawn)))
  (bind _returnvalue (- _returnvalue_z_2 1500.0))
  (if (<= _returnvalue_z _returnvalue)
    ;;[1 1 1 1 11] If the player is over 1000 feet above the lava, the lava respositions itself to keep up witht the player, while reseting its speed.
    (`self.K2_SetActorLocation` (`KismetMathLibrary.MakeVector` 0.0 0.0 _returnvalue))
    (set `self.speed` 0.0)
    (else
      ;;[1 1 1 1 11] If the lava is relatively close to the player, it gradually picks up speed to punish the player for not moving. No camping!
      (bind _output_get (set `self.speed` (+ (`self.speed`) DeltaSeconds)))
      (`self.K2_AddActorWorldTransform` (`KismetMathLibrary.MakeTransform` (`KismetMathLibrary.MakeVector` 0.0 0.0 _output_get))))))

(fn `UserConstructionScript`)